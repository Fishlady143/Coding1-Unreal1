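; BP_SpawnManager spawns waves of BP_Enemy actors at every BP_SpawnPoint in the level.
; BeginPlay triggers the first wave after a short random delay, and each enemy takes its spawn point's location and rotation with a random non-uniform scale.
; WaveCheck, which nothing in this Blueprint calls, starts another wave after a fixed delay when at most one enemy remains.
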(event Custom|SpawnEnemies
  (bind _outactors (Actor|GetAllActorsOfClass "/Game/Blueprints/BP_SpawnPoint.BP_SpawnPoint_C"))
  (for (_array_element _array_index) _outactors
    (Development|PrintString (Utilities|String|ToString(Integer) _array_index))
    (Game|SpawnActorfromClass "/Game/Blueprints/BP_Enemy.BP_Enemy_C" (Math|Transform|MakeTransform (.location (Transformation|GetActorTransform _array_element)) (.rotation (Transformation|GetActorTransform _array_element)) (Math|Vector|MakeVector (Math|Random|RandomFloatinRange 0.3 3.0) (Math|Random|RandomFloatinRange 0.3 3.0) (Math|Random|RandomFloatinRange 0.3 3.0))) "Undefined" "MultiplyWithRoot" 0 0))
  (Development|PrintString "Wowee!"))

(event Custom|WaveCheck
  (bind _outactors (Actor|GetAllActorsOfClass "/Game/Blueprints/BP_Enemy.BP_Enemy_C"))
  (if (> (Utilities|Array|Length _outactors) 1)
    (Development|PrintString "Not the last")
    (else
      (Utilities|FlowControl|Delay 5.0)
      (CallFunction|SpawnEnemies))))

(event EventBeginPlay
  (Development|PrintString "what if we kissed >.<" true true "(R=1.000000,G=0.833333,B=0.000000,A=1.000000)")
  (Utilities|FlowControl|Delay (Math|Random|RandomFloatinRange 0.1 5.0))
  (CallFunction|SpawnEnemies))

(fn ConstructionScript)