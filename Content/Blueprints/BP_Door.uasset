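; BP_Door is a key-locked door that opens when the player character hits it while holding at least one key.
; A hit on its Cube casts the other actor to BP_CustomTPChar, spends one key from TotalKeys and prints the remaining count.
; The SlideOpen timeline then sinks the door by a fixed local offset on each update, so travel depends on frame rate, and destroys the actor when finished.
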(event OnComponentHit(Cube)
  (params (HitComponent :type Primitive%20Component%20Object%20Reference) (OtherActor :type Actor%20Object%20Reference) (OtherComp :type Primitive%20Component%20Object%20Reference) (NormalImpulse :type Vector :default "0, 0, 0") (Hit :type Hit%20Result%20Structure%20%28by%20ref%29))
  (bind _asbp_custom_tpchar (Utilities|Casting|CastToBP_CustomTPChar OtherActor))
  (if (> (Variables|/Game/Blueprints/BP_CustomTPChar.BP_CustomTPChar_C|GetTotalKeys _asbp_custom_tpchar) 0)
    (Math|Integer|DecrementInt (Variables|/Game/Blueprints/BP_CustomTPChar.BP_CustomTPChar_C|GetTotalKeys _asbp_custom_tpchar)
      (:%20%20
        (Development|PrintString (Utilities|String|Append "You have " (Utilities|String|ToString(Integer) (Variables|/Game/Blueprints/BP_CustomTPChar.BP_CustomTPChar_C|GetTotalKeys _asbp_custom_tpchar)) " keys!"))
        (Timeline|Slide%20Open Play
          (:Update
            (Transformation|AddActorLocalOffset "0.000000,0.000000,-20.000000" false false))
          (:Finished
            (Actor|DestroyActor)))))))

(fn ConstructionScript)